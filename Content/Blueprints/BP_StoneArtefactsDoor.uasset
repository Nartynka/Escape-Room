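; A puzzle door that opens by destroying itself once both the Scarab and Ankh artefact interactions are completed.
; On BeginPlay it gathers each interaction component's required gameplay tag into an ItemsToActivate container.
; Each interaction removes its tag, reveals the matching artefact mesh and prints a debug message.
; CheckIfOpen then compares the remaining tags to an empty container and calls OpenDoor when they match.
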(event OnInteractDelegate(Scarab_IS)
  (bind _returnvalue (GameplayTags|RemoveGameplayTag (Variables|Default|GetItemsToActivate) (Variables|/Script/InteractionPlugin.InteractionSphere|GetRequiredTag (Variables|Default|GetScarab_IS)) :!class /Script/GameplayTags.BlueprintGameplayTagLibrary))
  (if _returnvalue
    (CallFunction|SpawnScarab)
    (CallFunction|CheckifOpen)))

(event OnInteractDelegate(Ankh_IS)
  (bind _returnvalue (GameplayTags|RemoveGameplayTag (Variables|Default|GetItemsToActivate) (Variables|/Script/InteractionPlugin.InteractionSphere|GetRequiredTag (Variables|Default|GetAnkh_IS)) :!class /Script/GameplayTags.BlueprintGameplayTagLibrary))
  (if _returnvalue
    (CallFunction|SpawnAnkh)
    (CallFunction|CheckifOpen)))

(event Custom|OpenDoor
  (Actor|DestroyActor))

(event Custom|SpawnScarab
  (Development|PrintString "Scarab Done!")
  (Rendering|SetVisibility (Variables|Default|GetSM_Scarab) true false))

(event Custom|SpawnAnkh
  (Development|PrintString "Ankh Done!")
  (Rendering|SetVisibility (Variables|Default|GetSM_Ankh) true false))

(event EventBeginPlay
  (bind _itemstoactivate (Variables|Default|GetItemsToActivate))
  (GameplayTags|AddGameplayTag _itemstoactivate (Variables|/Script/InteractionPlugin.InteractionSphere|GetRequiredTag (Variables|Default|GetScarab_IS)) :!class /Script/GameplayTags.BlueprintGameplayTagLibrary)
  (GameplayTags|AddGameplayTag _itemstoactivate (Variables|/Script/InteractionPlugin.InteractionSphere|GetRequiredTag (Variables|Default|GetAnkh_IS)) :!class /Script/GameplayTags.BlueprintGameplayTagLibrary))

(fn ConstructionScript)

(fn CheckifOpen
  (if (== (Variables|Default|GetItemsToActivate) (GameplayTags|MakeGameplayTagContainerfromTag))
    (CallFunction|OpenDoor)))