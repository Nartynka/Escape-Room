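; BP_Door is a door actor that slides its Cube back and forth in response to two buttons.
; On BeginPlay it binds a custom event to the interaction sphere event of each target, Button and Button2.
; Each interaction prints a debug message and instantly shifts the Cube along local X, in opposite directions per button, with no sweep, interpolation or position limit.
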(event Custom|CustomEvent_2
  (Development|PrintString "INTERACTION 2 RECIVED" true true "(R=0.091299,G=1.000000,B=0.575427,A=1.000000)")
  (Transformation|AddLocalOffset (Variables|Default|GetCube) "-100.000000,0.000000,0.000000" false false))

(event Custom|CustomEvent
  (Development|PrintString "INTERACTION RECIVED")
  (Transformation|AddLocalOffset (Variables|Default|GetCube) "100.000000,0.000000,0.000000" false false))

(event EventBeginPlay
  (CallFunction|BindEventonIntercttoInteractionSphere (Variables|Default|GetButton) (delegate Custom|CustomEvent))
  (CallFunction|BindEventonIntercttoInteractionSphere (Variables|Default|GetButton_2) (delegate Custom|CustomEvent_2)))

(fn ConstructionScript)