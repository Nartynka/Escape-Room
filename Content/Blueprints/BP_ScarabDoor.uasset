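; BP_ScarabDoor is a puzzle door that opens, by destroying itself, once the pink, blue and green scarabs are all activated.
; BeginPlay gathers each scarab interaction component's RequiredTag into the ItemsToActivate tag container.
; Each interaction removes its tag and, if successful, reveals the matching scarab mesh with a debug print.
; CheckIfOpen then compares the remaining tags against an empty container to trigger OpenDoor.
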(event OnInteractDelegate(GreenScarab_IS)
  (bind _returnvalue (GameplayTags|RemoveGameplayTag (Variables|Default|GetItemsToActivate) (Variables|/Script/InteractionPlugin.InteractionSphere|GetRequiredTag (Variables|Default|GetGreenScarab_IS)) :!class /Script/GameplayTags.BlueprintGameplayTagLibrary))
  (if _returnvalue
    (CallFunction|SpawnScarabGreen)
    (CallFunction|CheckifOpen)))

(event OnInteractDelegate(PinkScarab_IS)
  (bind _returnvalue (GameplayTags|RemoveGameplayTag (Variables|Default|GetItemsToActivate) (Variables|/Script/InteractionPlugin.InteractionSphere|GetRequiredTag (Variables|Default|GetPinkScarab_IS)) :!class /Script/GameplayTags.BlueprintGameplayTagLibrary))
  (if _returnvalue
    (CallFunction|SpawnScarabPink)
    (CallFunction|CheckifOpen)))

(event OnInteractDelegate(BlueScarab_IS)
  (bind _returnvalue (GameplayTags|RemoveGameplayTag (Variables|Default|GetItemsToActivate) (Variables|/Script/InteractionPlugin.InteractionSphere|GetRequiredTag (Variables|Default|GetBlueScarab_IS)) :!class /Script/GameplayTags.BlueprintGameplayTagLibrary))
  (if _returnvalue
    (CallFunction|SpawnScarabBlue)
    (CallFunction|CheckifOpen)))

(event Custom|SpawnScarabBlue
  (Development|PrintString "Spawn Blue")
  (Rendering|SetVisibility (Variables|Default|GetSM_ScarabBlue) true false))

(event Custom|SpawnScarabPink
  (Development|PrintString "Spawn Pink")
  (Rendering|SetVisibility (Variables|Default|GetSM_ScarabPink) true false))

(event Custom|SpawnScarabGreen
  (Development|PrintString "Spawn Green")
  (Rendering|SetVisibility (Variables|Default|GetSM_ScarabGreen) true false))

(event Custom|OpenDoor
  (Actor|DestroyActor))

(event EventBeginPlay
  (bind _itemstoactivate (Variables|Default|GetItemsToActivate))
  (GameplayTags|AddGameplayTag _itemstoactivate (Variables|/Script/InteractionPlugin.InteractionSphere|GetRequiredTag (Variables|Default|GetPinkScarab_IS)) :!class /Script/GameplayTags.BlueprintGameplayTagLibrary)
  (GameplayTags|AddGameplayTag _itemstoactivate (Variables|/Script/InteractionPlugin.InteractionSphere|GetRequiredTag (Variables|Default|GetBlueScarab_IS)) :!class /Script/GameplayTags.BlueprintGameplayTagLibrary)
  (GameplayTags|AddGameplayTag _itemstoactivate (Variables|/Script/InteractionPlugin.InteractionSphere|GetRequiredTag (Variables|Default|GetGreenScarab_IS)) :!class /Script/GameplayTags.BlueprintGameplayTagLibrary))

(fn ConstructionScript)

(fn CheckifOpen
  (if (== (Variables|Default|GetItemsToActivate) (GameplayTags|MakeGameplayTagContainerfromTag))
    (CallFunction|OpenDoor)))